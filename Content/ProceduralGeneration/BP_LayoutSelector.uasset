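; Procedural level spawner that builds layouts and backgrounds ahead of the player along the X axis.
; BeginPlay spawns a starting layout and background; CreateNew picks a random layout from the Low, Mid, High or Office pool by entry type.
; FindCharLoc derives the spawn X from player position and a 5000-unit segment length.
; A FlipFlop adds a random background on alternate calls, while cleanup functions shift previous/current/next references and destroy old actors.
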(event Custom|CreateNew
  (params (AccessEntry :type Integer))
  (bind _returnvalue (CallFunction|FindCharLoc))
  (bind _office (Variables|Default|GetOffice))
  (bind _mid (Variables|Default|GetMid))
  (bind _high (Variables|Default|GetHigh))
  (bind _low (Variables|Default|GetLow))
  (bind _returnvalue_2 (Math|Vector|MakeVector _returnvalue 0.0 0.0))
  ;[1 1 1] Spawn Layout
  (Development|PrintString (Utilities|String|ToString(Vector) (Transformation|GetWorldLocation (Variables|/Script/Engine.Character|GetMesh (Game|GetPlayerCharacter 0)))) true true "(R=0.101699,G=1.000000,B=0.000000,A=1.000000)")
  (switch int AccessEntry
    (:1
      (bind _returnvalue_3 (Game|SpawnActorfromClass (Utilities|Array|Get(acopy) _low (Math|Random|RandomInteger (Utilities|Array|Length _low))) (Math|Transform|MakeTransform _returnvalue_2 "0, 0, 0" "1.000000,1.000000,1.000000") "Undefined" "MultiplyWithRoot" 0 0))
      (CallFunction|LayoutCleanUp _returnvalue_3))
    (:2
      (bind _returnvalue_4 (Game|SpawnActorfromClass (Utilities|Array|Get(acopy) _mid (Math|Random|RandomInteger (Utilities|Array|Length _mid))) (Math|Transform|MakeTransform _returnvalue_2 "0, 0, 0" "1.000000,1.000000,1.000000") "Undefined" "MultiplyWithRoot" 0 0))
      (CallFunction|LayoutCleanUp _returnvalue_4))
    (:3
      (bind _returnvalue_5 (Game|SpawnActorfromClass (Utilities|Array|Get(acopy) _high (Math|Random|RandomInteger (Utilities|Array|Length _high))) (Math|Transform|MakeTransform _returnvalue_2 "0, 0, 0" "1.000000,1.000000,1.000000") "Undefined" "MultiplyWithRoot" 0 0))
      (CallFunction|LayoutCleanUp _returnvalue_5))
    (:4
      (bind _returnvalue_6 (Game|SpawnActorfromClass (Utilities|Array|Get(acopy) _office (Math|Random|RandomInteger (Utilities|Array|Length _office))) (Math|Transform|MakeTransform _returnvalue_2 "0, 0, 0" "1.000000,1.000000,1.000000") "Undefined" "MultiplyWithRoot" 0 0))
      (CallFunction|LayoutCleanUp _returnvalue_6)))
  (Utilities|FlowControl|FlipFlop
    (:B
      (bind _returnvalue_7 (Game|SpawnActorfromClass (.OutItem (Utilities|Array|Random (Variables|Default|GetBackgrounds))) (Math|Transform|MakeTransform (Math|Vector|MakeVector (CallFunction|FindCharLoc) -1e+02 0.0) "0, 0, 0" "1.000000,1.000000,1.000000") "Undefined" "MultiplyWithRoot" 0 0))
      (CallFunction|BackgroundCleanUp _returnvalue_7))))

(event EventBeginPlay
  ;[1 1 1] Spawn Starting
  (bind _returnvalue (Game|SpawnActorfromClass "/Game/ProceduralGeneration/Layouts/MidPlatforms/OfficeLow/BP_MidOfficeWindowExit.BP_MidOfficeWindowExit_C" (Math|Transform|MakeTransform "0, 0, 0" "0, 0, 0" "1.000000,1.000000,1.000000") "Undefined" "MultiplyWithRoot" 0 0))
  (Variables|Default|SetCurrLayout _returnvalue)
  (bind _returnvalue_2 (Game|SpawnActorfromClass "/Game/Background/Background1.Background1_C" (Math|Transform|MakeTransform "0.000000,-100.000000,0.000000" "0, 0, 0" "1.000000,1.000000,1.000000") "Undefined" "MultiplyWithRoot" 0 0))
  (Variables|Default|SetCurrBackground _returnvalue_2))

(fn ConstructionScript)

(fn LayoutCleanUp
  (params (NewLayout :type Actor%20Object%20Reference))
  (Utilities|IsValid (Variables|Default|GetNextLayout)
    (:Is%20Valid
      (Utilities|IsValid (Variables|Default|GetPrevLayout)
        (:Is%20Valid
          (Actor|DestroyActor (Variables|Default|GetPrevLayout)))
        (:Is%20Not%20Valid
          _))
      (Variables|Default|SetPrevLayout (Variables|Default|GetCurrLayout))
      (Variables|Default|SetCurrLayout (Variables|Default|GetNextLayout))
      (Variables|Default|SetNextLayout NewLayout))
    (:Is%20Not%20Valid
      (Variables|Default|SetNextLayout NewLayout))))

(fn FindCharLoc
  (return (* 5e+03 (+ 1 (/ (+ (.x (Transformation|GetActorLocation (Game|GetPlayerCharacter 0))) 5e+02) 5000)))))

(fn BackgroundCleanUp
  (params (NextBackground :type Actor%20Object%20Reference))
  (Utilities|IsValid (Variables|Default|GetNextBackground)
    (:Is%20Valid
      (Utilities|IsValid (Variables|Default|GetPrevBackground)
        (:Is%20Valid
          (Actor|DestroyActor (Variables|Default|GetPrevBackground)))
        (:Is%20Not%20Valid
          _))
      (Variables|Default|SetPrevBackground (Variables|Default|GetCurrBackground))
      (Variables|Default|SetCurrBackground (Variables|Default|GetNextBackground))
      (Variables|Default|SetNextBackground NextBackground))
    (:Is%20Not%20Valid
      (Variables|Default|SetNextBackground NextBackground))))
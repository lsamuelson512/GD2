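; BP_MidMaster is a mid-platform piece for procedural layouts that requests new layout generation when the player reaches it.
; On BeginPlay it caches the BP_LayoutSelector actor, then resets a DoOnce gate after a short delay.
; Box overlaps feed that gate, which then checks for the player character and calls CreateNew on the selector with AccessExit, plus a debug print.
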(event OnComponentBeginOverlap(Box)
  (params (OverlappedComponent :type Primitive%20Component%20Object%20Reference) (OtherActor :type Actor%20Object%20Reference) (OtherComp :type Primitive%20Component%20Object%20Reference) (OtherBodyIndex :type Integer) (bFromSweep :type Boolean) (SweepResult :type Hit%20Result%20Structure%20%28by%20ref%29))
  (Utilities|FlowControl|DoOnce false
    (:Completed
      (if (== OtherActor (Game|GetPlayerCharacter 0))
        (Default|CreateNew (Variables|Default|GetSelectorRef) (Variables|Default|GetAccessExit))
        (Development|PrintString "Hello")))))

(event EventBeginPlay
  (bind _returnvalue (Actor|GetActorOfClass "/Game/ProceduralGeneration/BP_LayoutSelector.BP_LayoutSelector_C"))
  (Variables|Default|SetSelectorRef _returnvalue)
  (Utilities|FlowControl|Delay 1.0)
  (Utilities|FlowControl|DoOnce false) ; enters at Reset
)

(fn ConstructionScript)